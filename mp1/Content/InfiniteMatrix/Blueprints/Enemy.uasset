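; Enemy obstacle actor that damages the player on contact in a forward-moving runner.
; Each tick it destroys itself once the player's sphere passes it along the X axis.
; Overlapping its mesh costs the player health, triggers a camera shake and destroys the enemy.
; When health runs out, it marks the player dead, resets position, score, count and speed, and shows the restart UI.
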(event OnComponentBeginOverlap(Medium_HP_Mk2)
  (params (OverlappedComponent :type Primitive%20Component%20Object%20Reference) (OtherActor :type Actor%20Object%20Reference) (OtherComp :type Primitive%20Component%20Object%20Reference) (OtherBodyIndex :type Integer) (bFromSweep :type Boolean) (SweepResult :type Hit%20Result%20Structure%20%28by%20ref%29))
  (bind _asbp_player (Utilities|Casting|CastToBP_Player OtherActor))
  (bind _output_get (Variables|/Game/InfiniteMatrix/Blueprints/BP_Player.BP_Player_C|SetHealth _asbp_player (- (Variables|/Game/InfiniteMatrix/Blueprints/BP_Player.BP_Player_C|GetHealth _asbp_player) 30)))
  (Game|Feedback|ClientStartCameraShake (Game|GetPlayerController 0) "/Game/InfiniteMatrix/Blueprints/Shake.Shake_C" 1e+01 "CameraLocal" "0, 0, 0")
  (Actor|DestroyActor)
  (Math|Integer|CompareInt _output_get
    (:==
      _)
    (:<
      _))
  (Variables|/Game/InfiniteMatrix/Blueprints/BP_Player.BP_Player_C|SetIsDead _asbp_player true)
  (Transformation|SetActorLocation _asbp_player "0, 0, 0" false false)
  (Variables|/Game/InfiniteMatrix/Blueprints/BP_Player.BP_Player_C|SetScore _asbp_player 0)
  (Variables|/Game/InfiniteMatrix/Blueprints/BP_Player.BP_Player_C|Setcount _asbp_player 0)
  (Variables|/Game/InfiniteMatrix/Blueprints/BP_Player.BP_Player_C|SetForwardSpeed _asbp_player 5e+02)
  (Default|DisplayRestart _asbp_player))

(event EventBeginPlay)

(event Collision|EventActorBeginOverlap
  (params (OtherActor :type Actor%20Object%20Reference)))

(event EventTick
  (params (DeltaSeconds :type Float%20%28single-precision%29))
  (bind _asbp_player (Utilities|Casting|CastToBP_Player (Game|Player|GetPlayerPawn 0)))
  (if (> (.x (Transformation|GetWorldLocation (Variables|/Game/InfiniteMatrix/Blueprints/BP_Player.BP_Player_C|GetSphere _asbp_player))) (+ (.x (Transformation|GetWorldLocation (Variables|Default|GetMedium_HP_Mk2 self))) 1e+02))
    (Actor|DestroyActor)))

(fn ConstructionScript)